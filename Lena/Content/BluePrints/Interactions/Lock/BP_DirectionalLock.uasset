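; BP_DirectionalLock is an interactable directional lock driven by the arrow keys.
; Each key press, ignored while a movement is in progress, calls MoveFromStart with an offset on X (right/left) or Z (up/down) and a direction code from "1" to "4".
; SetPassword appends a string to InputPassWord to build the entered code; no call to it or password check appears in these graphs.
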(event EventBeginPlay)

(event Collision|EventActorBeginOverlap
  (params (OtherActor :type Actor%20Object%20Reference)))

(event EventTick
  (params (DeltaSeconds :type Float%20%28single-precision%29)))

(event Input|KeyboardEvents|Right
  (params (Key :type Key%20Structure))
  ;[1 1 1] 1
  (:Pressed
    (bind _returnvalue (Class|DirectionalLockActor|IsMovementProgressing))
    (if (not _returnvalue)
      (Class|DirectionalLockActor|MovefromStart "7.000000,0.000000,0.000000" (Utilities|String|ToString(Integer) (Class|KismetSystemLibrary|MakeLiteralInteger 1))))))

(event Input|KeyboardEvents|Left
  (params (Key :type Key%20Structure))
  ;[1 1 1] 2
  (:Pressed
    (bind _returnvalue (Class|DirectionalLockActor|IsMovementProgressing))
    (if (not _returnvalue)
      (Class|DirectionalLockActor|MovefromStart "-7.000000,0.000000,0.000000" (Utilities|String|ToString(Integer) (Class|KismetSystemLibrary|MakeLiteralInteger 2))))))

(event Input|KeyboardEvents|Up
  (params (Key :type Key%20Structure))
  ;[1 1 1] 3
  (:Pressed
    (bind _returnvalue (Class|DirectionalLockActor|IsMovementProgressing))
    (if (not _returnvalue)
      (Class|DirectionalLockActor|MovefromStart "0.000000,0.000000,7.000000" (Utilities|String|ToString(Integer) (Class|KismetSystemLibrary|MakeLiteralInteger 3))))))

(event Input|KeyboardEvents|Down
  (params (Key :type Key%20Structure))
  ;[1 1 1] 4
  (:Pressed
    (bind _returnvalue (Class|DirectionalLockActor|IsMovementProgressing))
    (if (not _returnvalue)
      (Class|DirectionalLockActor|MovefromStart "0.000000,0.000000,-7.000000" (Utilities|String|ToString(Integer) (Class|KismetSystemLibrary|MakeLiteralInteger 4))))))

(fn ConstructionScript)

(fn SetPassword
  (params (NewParam :type String))
  (Variables|Default|SetInputPassWord (Utilities|String|Append (Variables|Default|GetInputPassWord) NewParam)))