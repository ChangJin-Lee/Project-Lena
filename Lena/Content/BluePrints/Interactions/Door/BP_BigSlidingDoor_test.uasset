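; Test version of a big sliding door that is opened through a numpad widget.
; Until the door is done, pressing E alternately shows and removes the numpad from its widget component, and an outside event also removes it.
; The open-door interface event slides the door along negative X, marks it done and removes the numpad.
; An OpenDoorTimeLine node is left unconnected.
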(event Custom|BPI_OpenDoorEvent
  (Class|SlidingDoorActor|OpenSlidingDoor "-400.000000,0.000000,0.000000")
  (Variables|Default|SetIsDone true)
  (Class|InteractableActor|RemoveWidget (UserInterface|GetWidget (Variables|Default|GetNumpadWidgetComponent))))

(event EventOutSideEvent
  (Class|InteractableActor|RemoveWidget (UserInterface|GetWidget (Variables|Default|GetNumpadWidgetComponent))))

(event Input|KeyboardEvents|E
  (params (Key :type Key%20Structure))
  (bind _numpadwidgetcomponent (Variables|Default|GetNumpadWidgetComponent))
  (bind _returnvalue (UserInterface|GetWidget _numpadwidgetcomponent))
  (:Pressed
    (if (not (Variables|Default|GetIsDone))
      (Utilities|FlowControl|FlipFlop
        (:A
          (Class|InteractableActor|AddWidget _returnvalue))
        (:B
          (Class|InteractableActor|RemoveWidget _returnvalue))))))

(fn ConstructionScript)