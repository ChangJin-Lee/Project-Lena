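; Hinged door actor that opens on the E key only when the level's button lock holds the correct code.
; E checks the first BP_ButtonLock found against a hardcoded password, then hides the lock's widget, plays a sound and calls OpenHingedDoor.
; On failure it plays the close sound and changes its interact prompt to ask for the lock to be solved.
; Closing logic and an OpenLock call are left unconnected.
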(event EventBeginPlay
  (bind _asinteract_widget (Utilities|Casting|CastToInteractWidget (UserInterface|GetWidget (Variables|Default|GetWidgetComponent))))
  (Class|InteractWidget|SetInstructionatBeginPlay _asinteract_widget "Press E to Open Door"))

(event Collision|EventActorBeginOverlap
  (params (OtherActor :type Actor%20Object%20Reference)))

(event EventTick
  (params (DeltaSeconds :type Float%20%28single-precision%29)))

(event Input|KeyboardEvents|E
  (params (Key :type Key%20Structure :default "None"))
  (:Pressed
    (bind _outactors (Actor|GetAllActorsOfClass "/Game/BluePrints/Interactions/Lock/BP_ButtonLock.BP_ButtonLock_C"))
    (bind _returnvalue (Class|ButtonLockActor|ValidPassword (Utilities|Array|Get(acopy) _outactors) "1367"))
    (if _returnvalue
      (Widget|SetVisibility (UserInterface|GetWidget (Variables|/Script/Lena.InteractableActor|GetWidgetComponent (Utilities|Array|Get(acopy) _outactors))) "Hidden")
      (Audio|PlaySoundatLocation "/Game/SFX/Hinged_Door_Open.Hinged_Door_Open" "0, 0, 0" "0, 0, 0" 1.0 1.0 0.0 0 0 0 0)
      (Class|HingedDoorActor|OpenHingedDoor "0.000000,-90.000000,0.000000")
      (else
        (Audio|PlaySoundatLocation "/Game/SFX/Hinged_Door_Close.Hinged_Door_Close" "0, 0, 0" "0, 0, 0" 1.0 1.0 0.0 0 0 0 0)
        (Class|InteractWidget|SetInstruction (stale EventBeginPlay _asinteract_widget) "Please Solve Button Lock")))))

(fn ConstructionScript)