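; BP_SlidingDoor1 is an interactable sliding door that opens on the E key when a required-item check passes.
; On success, a timeline drives the mesh's relative location, and each update sets IsDone and removes the widget.
; On failure, the text render flashes the wrong-answer color for half a second and a world camera shake plays.
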(event Input|KeyboardEvents|E
  (params (Key :type Key%20Structure :default "None"))
  (:Pressed
    (bind _returnvalue (Class|DoorActor|CheckRequiredItem))
    (if _returnvalue
      (bind _새_트랙_0 (Timeline|OpenDoorTimeLine Play)
        (:Update
          (Transformation|SetRelativeLocation (Variables|Default|GetMeshComponent) _새_트랙_0 false false)
          (Variables|Default|SetIsDone true)
          (Class|InteractableActor|RemoveWidget)))
      (else
        (Rendering|Components|TextRender|SetTextRenderColor (Variables|Default|GetTextRenderComponent) (Variables|Default|GetWrongAnswerColor))
        (Camera|PlayWorldCameraShake 0 "1.000000,1.000000,1.000000" 0.0 0.0)
        (Utilities|FlowControl|Delay 0.5)
        (Rendering|Components|TextRender|SetTextRenderColor (Variables|Default|GetTextRenderComponent) (Variables|Default|GetDefaultAnswerColor))))))

(fn ConstructionScript)