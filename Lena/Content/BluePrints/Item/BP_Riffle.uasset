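; BP_Riffle is a rifle item actor that sets up its M4A1 skeletal mesh and a separate magazine on BeginPlay.
; A SceneCapture2D is limited to that mesh and captures it before the M4A1 asset is assigned.
; A collision-free static mesh component is then created, stored as OldMag and snapped to the "mag" socket, while the built-in magazine bone is hidden.
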(event EventBeginPlay
  (Rendering|SceneCapture|ShowOnlyComponent (Variables|Default|GetSceneCaptureComponent2D) (Variables|Character|GetMesh))
  (Rendering|SceneCapture|CaptureScene (Variables|Default|GetSceneCaptureComponent2D) :!class /Script/Engine.SceneCaptureComponent2D)
  (Components|SkeletalMesh|SetSkeletalMeshAsset (Variables|Character|GetMesh) "/Game/Props/Meshes/M4A1.M4A1")
  (bind _returnvalue (AddComponent|AddStaticMeshComponent false))
  (Collision|SetCollisionEnabled _returnvalue "NoCollision")
  (bind _output_get (Variables|Default|SetOldMag _returnvalue))
  (Transformation|AttachComponentToComponent _output_get (Variables|Character|GetMesh) "mag" "SnapToTarget" "SnapToTarget" "KeepRelative" true)
  (Components|SkinnedMesh|HideBonebyName (Variables|Character|GetMesh) "magazine" "PBO_None"))

(event Collision|EventActorBeginOverlap
  (params (OtherActor :type Actor%20Object%20Reference)))

(event EventTick
  (params (DeltaSeconds :type Float%20%28single-precision%29)))

(fn ConstructionScript)