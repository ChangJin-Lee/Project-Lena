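; Sliding door actor that opens through a timeline, with a widget toggled by the E key.
; OpenTheDoor plays the timeline, feeding its track into MoveDoor on each update.
; E flip-flops between AddWidget and RemoveWidget, while OutSideEvent shows a TextRender and also removes the widget.
; An unconnected older branch creates WBP_Numpad directly and switches input mode and mouse cursor.
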(event Custom|Open%20The%20Door
  (bind _새_트랙_0 (Timeline|타임라인 Play)
    (:Update
      (Class|SlidingDoor|MoveDoor _새_트랙_0))))

(event EventBeginPlay)

(event Collision|EventActorBeginOverlap
  (params (OtherActor :type Actor%20Object%20Reference)))

(event EventTick
  (params (DeltaSeconds :type Float%20%28single-precision%29)))

(event EventOutSideEvent
  (Rendering|SetVisibility (Variables|Default|GetTextRender) true false)
  (Class|SlidingDoor|RemoveWidget))

(event Input|KeyboardEvents|E
  (params (Key :type Key%20Structure :default "None"))
  (:Pressed
    (Utilities|FlowControl|FlipFlop
      (:A
        (Class|SlidingDoor|AddWidget))
      (:B
        (Class|SlidingDoor|RemoveWidget)))))

(fn ConstructionScript)

(fn NewFunction
  (return (Variables|Default|GetGetAround)))